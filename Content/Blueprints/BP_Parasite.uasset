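; BP_Parasite is a parasite actor that shows a health bar, using a BP_Enemy_Health widget in its EnemyHealth component.
; BeginPlay casts and caches the widget reference.
; Every tick sets the progress bar from Health on a 100-point scale and rotates the widget component to face the player camera, billboard style.
; The overlap event and construction script are empty.
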(event `self.ReceiveBeginPlay`
  (bind _asbp_enemy_health (cast `/Game/UI/BP_Enemy_Health` (`WidgetComponent.GetUserWidgetObject` (`self.Enemy health`))))
  (set `self.enemy health ui ref` _asbp_enemy_health))

(event `self.ReceiveTick`
  (params (DeltaSeconds :type "Float (single-precision)"))
  (bind _enemy_health (`self.Enemy health`))
  (`ProgressBar.SetPercent` (`/Game/UI/BP_Enemy_Health.ProgressBar_0` (`self.enemy health ui ref`)) (/ (`self.Health`) 100.0))
  (`SceneComponent.K2_SetWorldRotation` _enemy_health (`KismetMathLibrary.FindLookAtRotation` (`SceneComponent.K2_GetComponentLocation` _enemy_health) (`SceneComponent.K2_GetComponentLocation` (`PlayerCameraManager.TransformComponent` (`GameplayStatics.GetPlayerCameraManager` 0)))) false false))

(fn `UserConstructionScript`)