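; BP_Mutant is a mutant enemy Blueprint that shows its health on a floating widget bar.
; On BeginPlay it casts the MutantHealth component's widget to BP_Mutant_UI and caches it.
; Each Tick it sets the bar's percent from Health over a fixed maximum and rotates the widget toward the player camera, billboard style.
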(event `self.ReceiveBeginPlay`
  (bind _asbp_mutant_ui (cast `/Game/UI/BP_Mutant_UI` (`WidgetComponent.GetUserWidgetObject` (`self.Mutant Health`))))
  (set `self.As BP Mutant UI` _asbp_mutant_ui))

(event `self.ReceiveTick`
  (params (DeltaSeconds :type "Float (single-precision)"))
  (bind _mutant_health (`self.Mutant Health`))
  (`ProgressBar.SetPercent` (`/Game/UI/BP_Mutant_UI.Mutant_HealthBar` (`self.As BP Mutant UI`)) (/ (`self.Health`) 500.0))
  (`SceneComponent.K2_SetWorldRotation` _mutant_health (`KismetMathLibrary.FindLookAtRotation` (`SceneComponent.K2_GetComponentLocation` _mutant_health) (`SceneComponent.K2_GetComponentLocation` (`PlayerCameraManager.TransformComponent` (`GameplayStatics.GetPlayerCameraManager` 0)))) false false))

(fn `UserConstructionScript`)