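; BP_Zombie is a zombie Blueprint that displays its health on an attached world widget.
; BeginPlay casts the ZombieHealth component's widget to BP_Zombie_Ui and caches the reference.
; Every Tick sets that widget's health bar from Health over a hard-coded maximum and rotates the component to face the player camera, billboard style.
; The overlap event is empty, and no damage or movement logic appears in these graphs.
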(event `self.ReceiveBeginPlay`
  (bind _asbp_zombie_ui (cast `/Game/UI/BP_Zombie_Ui` (`WidgetComponent.GetUserWidgetObject` (`self.Zombie_Health`))))
  (set `self.zombie health ref` _asbp_zombie_ui))

(event `self.ReceiveTick`
  (params (DeltaSeconds :type "Float (single-precision)"))
  (bind _zombie_health (`self.Zombie_Health`))
  (`ProgressBar.SetPercent` (`/Game/UI/BP_Zombie_Ui.Zombie_HealthBar` (`self.zombie health ref`)) (/ (`self.Health`) 500.0))
  (`SceneComponent.K2_SetWorldRotation` _zombie_health (`KismetMathLibrary.FindLookAtRotation` (`SceneComponent.K2_GetComponentLocation` _zombie_health) (`SceneComponent.K2_GetComponentLocation` (`PlayerCameraManager.TransformComponent` (`GameplayStatics.GetPlayerCameraManager` 0)))) false false))

(fn `UserConstructionScript`)